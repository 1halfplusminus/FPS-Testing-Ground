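; AI controller that runs a guard behavior tree on the PatrolData blackboard.
; Each tick it sets the controlled Character's Aiming and Shooting flags according to whether a focus actor is valid.
; The AI perception update event is empty, and a debug print of the sensed stimulus class is left disconnected.
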(event `self.ReceiveBeginPlay`
  (`self.UseBlackboard` "/Game/Character/AI/PatrolData.PatrolData")
  (`self.RunBehaviorTree` "/Game/Character/AI/GuardBehaviour.GuardBehaviour"))

(event `self.ReceiveTick`
  (params (DeltaSeconds :type "Float (single-precision)"))
  (bind _returnvalue (`KismetSystemLibrary.IsValid` (`self.GetFocusActor`)))
  (bind _ascharacter (cast `/Game/Character/Character` (`self.K2_GetPawn`)))
  (set `/Game/Character/Character.Aiming` _returnvalue _ascharacter)
  (set `/Game/Character/Character.Shooting` _returnvalue _ascharacter))

(event `self.AIPerception.OnTargetPerceptionUpdated`
  (params (Actor :type "Actor Object Reference") (Stimulus :type "AIStimulus Structure")))

(fn `UserConstructionScript`)