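; BP_Tile is a terrain tile for an infinite-terrain game that fills itself with randomized props, rocks and AI characters on BeginPlay.
; Inherited-style placement calls take spawn parameters for count ranges, collision radius and transform limits.
; Player-filtered trigger volumes lock a red barrier on entry, then turn it green, passable and report the tile conquered.
; Leaving the destroy volume asks the game mode for a new tile and destroys this one.
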(event `self.ReceiveBeginPlay`
  (bind (_rotation _scale) (break `SpawnPosition` (`self.MinTransform`)))
  (bind _spawnparams (make `SpawnParams` 3 8 100.0 (make `SpawnPosition` _rotation _scale) (make `SpawnPosition` (`.Rotation` (break `SpawnPosition` (`self.MaxTransform`))) (4.0 4.0 4.0))))
  (`self.PlaceActors` "/Game/Terrain/Props/BP_Container.BP_Container_C" (make `SpawnParams` 1 3 400.0 (`self.MinTransform`) (`self.MaxTransform`)))
  (`self.PlaceActors` "/Game/Terrain/Props/BP_Box.BP_Box_C" (make `SpawnParams` 2 4 100.0 (`self.MinTransform`) (`self.MaxTransform`)))
  (`self.PlaceActors` "/Game/Terrain/Props/BP_Canister.BP_Canister_C" (make `SpawnParams` 1 4 50.0 (`self.MinTransform`) (`self.MaxTransform`)))
  (`self.PlaceActors` "/Game/Terrain/Props/BP_Rock_01.BP_Rock_01_C" _spawnparams)
  (`self.PlaceActors` "/Game/Terrain/Props/BP_Rock_02.BP_Rock_02_C" _spawnparams)
  (`self.PlaceAIPawns` "/Game/Character/BP_Character.BP_Character_C" (make `SpawnParams` 1 4 100.0)))

(event `self.Locking Volume.OnComponentBeginOverlap`
  (params (OverlappedComponent :type "PrimitiveComponent Object Reference") (OtherActor :type "Actor Object Reference") (OtherComp :type "PrimitiveComponent Object Reference") (OtherBodyIndex :type Integer) (bFromSweep :type Boolean) (SweepResult :type "HitResult Structure (by ref)"))
  (`self.Is Player` OtherActor)
  (`self.Lock`))

(event `self.Opening Volume.OnComponentEndOverlap`
  (params (OverlappedComponent :type "PrimitiveComponent Object Reference") (OtherActor :type "Actor Object Reference") (OtherComp :type "PrimitiveComponent Object Reference") (OtherBodyIndex :type Integer))
  (`self.Is Player` OtherActor)
  (`self.UnLock`)
  (`self.TileConquered`))

(event `self.Destroy Volume.OnComponentEndOverlap`
  (params (OverlappedComponent :type "PrimitiveComponent Object Reference") (OtherActor :type "Actor Object Reference") (OtherComp :type "PrimitiveComponent Object Reference") (OtherBodyIndex :type Integer))
  (`self.Is Player` OtherActor)
  (bind _asbp_infinite_terrain_game_mode (cast `/Game/Core/BP_InfiniteTerrainGameMode` (`GameplayStatics.GetGameMode`)))
  (`TestingGroundGameMode.SpawnTile` _asbp_infinite_terrain_game_mode)
  (`self.K2_DestroyActor`))

(event `self.UnLock`
  (`PrimitiveComponent.SetCollisionEnabled` (`self.Barrier`) "NoCollision")
  (`PrimitiveComponent.SetMaterial` (`self.Barrier`) 0 "/Game/Terrain/MI_Barrier_Green.MI_Barrier_Green"))

(event `self.Lock`
  (`PrimitiveComponent.SetCollisionEnabled` (`self.Barrier`) "QueryAndPhysics")
  (`PrimitiveComponent.SetMaterial` (`self.Barrier`) 0 "/Game/Terrain/MI_Barrier_Red.MI_Barrier_Red"))

(fn `UserConstructionScript`)